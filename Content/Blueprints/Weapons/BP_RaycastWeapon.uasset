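; Hitscan weapon Blueprint that fires line traces, spends ammo and damages the hit actor.
; CEStartFire and CEStopFire drive a Gate, which re-enters after a Cadence delay for automatic fire while ammo remains.
; Traces run from the muzzle socket to a Range point along the owner's forward vector, not the camera view, with debug drawing on.
; Each shot plays sound, owner montage and muzzle particle, but no impact effect.
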(event `self.CE_StartFire`
  (bind (_startpoint _endpoint) (`self.F_StartAndEndPoint`))
  (bind _ownerreference (`self.OwnerReference`))
  (`|ExecutionSequence`
    (:`then_0`
      (goto _label :!via `Open`))
    (:`then_1`
      (`/Engine/EditorBlueprintResources/StandardMacros.Gate` true :!label _label
        (:`Exit`
          (if (> (`self.Ammo`) 0)
            (bind _outhit (`KismetSystemLibrary.LineTraceSingle` _startpoint _endpoint "TraceTypeQuery3" false (`|MakeArray` (`self.OwnerReference`) :!type "Actor Object Reference") "ForDuration"))
            (`self.F_DecrementAmmo`)
            (bind (_bblockinghit _binitialoverlap _time _distance _location _impactpoint _normal _impactnormal _physmat _hitactor _hitcomponent _hitbonename _bonename _hititem _elementindex _faceindex _tracestart _traceend) (`GameplayStatics.BreakHitResult` _outhit))
            (`self.F_PlayGunFX` _impactpoint (select `bool` _bblockinghit :`false` _traceend :`true` _impactpoint))
            (`GameplayStatics.ApplyDamage` _hitactor (`self.Damage`) (`self.GetInstigatorController` _ownerreference) _ownerreference)
            (if (`self.IsAuto`)
              (`KismetSystemLibrary.Delay` (`self.Cadence`))
              (goto _label))))))))

(event `self.CE_StopFire`
  (goto _label :!via `Close`))

(fn `F_DecrementAmmo`
  (`/Engine/EditorBlueprintResources/StandardMacros.DecrementInt` (`self.Ammo`)
    (:`  `
      (return))))

(fn `F_GetMuzzlePosition`
  (returns (MuzzlePosition :type "Vector Structure"))
  (bind _output_get (set `self.MuzzlePosition` (`SceneComponent.GetSocketLocation` (`self.SkeletalMesh`) "Muzzle")))
  (return _output_get))

(fn `F_PlayGunFX`
  (params (ImpactPoint :type "Vector Structure") (TraceEnd :type "Vector Structure"))
  (`GameplayStatics.PlaySoundAtLocation` (`self.Sound`) (`self.MuzzlePosition`) (struct) 0.2 1.0 0.0 null null null null)
  (`Character.PlayAnimMontage` (`self.OwnerReference`) (`self.ShootAnimation`) 1.0 "None")
  (`GameplayStatics.SpawnEmitterAttached` (`self.MuzzleParticle`) (`self.SkeletalMesh`) "Muzzle" (`self.MuzzlePosition`) (struct) (1.0 1.0 1.0) "SnapToTargetIncludingScale"))

(fn `F_StartAndEndPoint`
  (returns (StartPoint :type "Vector Structure") (EndPoint :type "Vector Structure"))
  (bind _rootcomponent (`Actor.RootComponent` (`self.OwnerReference`)))
  (bind _muzzleposition (`self.F_GetMuzzlePosition`))
  (return _muzzleposition (+ (`SceneComponent.K2_GetComponentLocation` _rootcomponent) (* (`KismetMathLibrary.GetForwardVector` (`SceneComponent.K2_GetComponentRotation` _rootcomponent)) (`self.Range`)))))

(fn `UserConstructionScript`
  (`parent.UserConstructionScript`))